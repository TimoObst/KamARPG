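; Example fireball projectile for the KamARPG ability system, with particle effects and a follow-up ability on kills.
; It spawns a shockwave effect on creation and a scaled-down explosion at each unit it hits.
; A kill chains BP_Firenado_Example from the killed unit.
; On destroy it runs the parent logic, then cuts its speed to a quarter and disables collision.
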(event `self.OnHit`
  (params (target :type "KamUnit Object Reference"))
  (bind _returnvalue (`KamUnit.GetUnitTransform` target))
  (`self.SpawnEmitterAtTransform` "/Game/FXVarietyPack/Particles/P_ky_explosion.P_ky_explosion" (`KismetMathLibrary.MakeTransform` (.location _returnvalue) (.rotation _returnvalue) (0.3 0.3 0.3))))

(event `self.OnKill`
  (params (target :type "KamUnit Object Reference"))
  (`self.ChainAbilityFromUnit` "/Game/KamARPG_Example/Abilities/Area/BP_Firenado_Example.BP_Firenado_Example_C" target))

(event `self.OnCreate`
  (`self.SpawnEmitterAtTransform` "/Game/FXVarietyPack/Particles/P_ky_shotShockwave.P_ky_shotShockwave"))

(event `self.OnDestroy`
  (`parent.OnDestroy`)
  (`self.SetSpeed` (/ (`self.Speed`) 4.0))
  (`self.SetActorEnableCollision` false))

(fn `UserConstructionScript`
  (`parent.UserConstructionScript`))