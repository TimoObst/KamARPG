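; Example Firenado area ability that periodically spawns fireballs in random directions.
; On each update it accumulates delta time and, whenever the timer reaches ChainFireballTime, chains a BP_KamFireball_Example projectile at a random angle, passing -1 for size, speed and distance.
; The interval is then subtracted rather than the timer reset, so leftover time carries into the next shot.
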(event `self.OnUpdate`
  (params (deltaTime :type "Float (single-precision)"))
  (bind _output_get (set `self.Timer` (+ deltaTime (`self.Timer`))))
  (if (>= _output_get (`self.ChainFireballTime`))
    (`self.ChainProjectile` "/Game/KamARPG_Example/Abilities/Projectiles/BP_KamFireball_Example.BP_KamFireball_Example_C" -1.0 (`KismetMathLibrary.RandomFloatInRange` 0.0 360.0) -1.0 -1.0)
    (set `self.Timer` (- (`self.Timer`) (`self.ChainFireballTime`)))))

(fn `UserConstructionScript`
  (`parent.UserConstructionScript`))