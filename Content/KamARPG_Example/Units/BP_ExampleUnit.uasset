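; BP_ExampleUnit is an example KamARPG unit that reacts visually to taking damage and tracks its attacked and dead states.
; On BeginPlay it binds to the damage-taken and death events of KamEnemyUnit.
; Positive damage picks a material flash color by damage element, plays a timeline that drives FlashAlpha on the skeletal mesh, and sets IsAttacked.
; Death only sets the IsDead flag.
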(event `self.ReceiveBeginPlay`
  (bind _kam_enemyunit (`self.Kam_EnemyUnit`))
  (add `KamUnit.OnDamageTakenEvent` _kam_enemyunit (delegate `On Damage Taken`))
  (add `KamUnit.OnDeathEvent` _kam_enemyunit (delegate `On Death`)))

(event `On Damage Taken`
  (params (damageTaken :type "Float (double-precision)") (damageElement :type "EKamElement Enum" :default "EL_True") (isCrit :type Boolean))
  (bind _skeletalmesh (`self.SkeletalMesh`))
  (if (> damageTaken 0.0)
    (switch `EKamElement` damageElement
      (:`EL_True`
        (`MeshComponent.SetVectorParameterValueOnMaterials` _skeletalmesh "FlashColor" (1.0 1.0 1.0)))
      (:`EL_Physical`
        (`MeshComponent.SetVectorParameterValueOnMaterials` _skeletalmesh "FlashColor" (1.0 0.0 0.0)))
      (:`EL_Magic`
        (`MeshComponent.SetVectorParameterValueOnMaterials` _skeletalmesh "FlashColor" (1.0 0.0 1.0)))
      (:`EL_Fire`
        (`MeshComponent.SetVectorParameterValueOnMaterials` _skeletalmesh "FlashColor" (10.0 0.0 0.0))))
    (`self.FlashColor`)
    (set `self.IsAttacked` true)))

(event `On Death`
  (set `self.IsDead` true))

(event `FlashColor`
  (bind (_direction _alpha) (`Timeline|FlashColorTimeline` :!via `PlayFromStart`)
    (:`Update`
      (`MeshComponent.SetScalarParameterValueOnMaterials` (`self.SkeletalMesh`) "FlashAlpha" _alpha))))

(fn `UserConstructionScript`)