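; BP_DarkStorm is a KamARPG ability projectile that grows as it travels and bursts into fireballs on hit.
; Spawn plays a small thunder-ball effect, and tick scales size and the registered particle system with distance traveled.
; Each hit plays that effect, chains six BP_Fireball projectiles at 60-degree intervals, and resets EnemiesHit.
; Destruction deactivates particles and sets a fixed speed, delaying removal until the system finishes.
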(event `self.OnCreate`
  (bind (_returnvalue_location _returnvalue_rotation) (`KismetMathLibrary.BreakTransform` (`self.GetTransform`)))
  (`self.SpawnParticleAtTransform` "/Game/FXVarietyPack/Particles/P_ky_ThunderBallHit.P_ky_ThunderBallHit" (`KismetMathLibrary.MakeTransform` _returnvalue_location _returnvalue_rotation (0.3 0.3 0.3)))
  (set `self.BaseSize` (`self.Size`)))

(event `self.OnTick`
  (params (deltaTime :type "Float (single-precision)"))
  (`self.SetSize` (+ (`self.BaseSize`) (* 0.8 (/ (`self.Distance`) (`self.MaxDistance`))))))

(event `self.OnDestroy`
  (`ActorComponent.Deactivate` (`self.ParticleSystem`))
  (`self.SetSpeed` 200.0))

(event `self.ParticleSystem.OnSystemFinished`
  (params (PSystem :type "ParticleSystemComponent Object Reference"))
  (`self.SetDelayDestroy` false))

(event `self.OnHit`
  (params (target :type "KamUnit Object Reference"))
  (`self.SpawnParticleAtUnit` "/Game/FXVarietyPack/Particles/P_ky_ThunderBallHit.P_ky_ThunderBallHit" target)
  (`self.ChainProjectileFromUnit` "/Game/KamARPG/Abilities/Projectiles/BP_Fireball.BP_Fireball_C" target)
  (`self.ChainProjectileFromUnit` "/Game/KamARPG/Abilities/Projectiles/BP_Fireball.BP_Fireball_C" target 0.0 60.0)
  (`self.ChainProjectileFromUnit` "/Game/KamARPG/Abilities/Projectiles/BP_Fireball.BP_Fireball_C" target 0.0 120.0)
  (`self.ChainProjectileFromUnit` "/Game/KamARPG/Abilities/Projectiles/BP_Fireball.BP_Fireball_C" target 0.0 180.0)
  (`self.ChainProjectileFromUnit` "/Game/KamARPG/Abilities/Projectiles/BP_Fireball.BP_Fireball_C" target 0.0 240.0)
  (`self.ChainProjectileFromUnit` "/Game/KamARPG/Abilities/Projectiles/BP_Fireball.BP_Fireball_C" target 0.0 300.0)
  (set `self.EnemiesHit` 0))

(fn `UserConstructionScript`
  (`parent.UserConstructionScript`)
  (`self.AddComponentToScale` (`self.ParticleSystem`))
  (`self.SetDelayDestroy` true))