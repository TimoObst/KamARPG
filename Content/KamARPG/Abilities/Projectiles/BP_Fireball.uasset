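; BP_Fireball is a fireball projectile ability that chains BP_FireNado from any unit it kills.
; It emits a shockwave on creation and a scaled-down explosion on each hit and on destroy.
; On destroy it stops moving, disables collision and deactivates its particle system, clearing the delayed-destroy flag when that system finishes.
; The construction script registers Collision for deactivation during delayed destruction.
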(event `self.OnKill`
  (params (target :type "KamUnit Object Reference"))
  (`self.ChainAbilityFromUnit` "/Game/KamARPG/Abilities/Area/BP_FireNado.BP_FireNado_C" target))

(event `self.OnHit`
  (params (target :type "KamUnit Object Reference"))
  (bind _returnvalue (`KamUnit.GetUnitTransform` target))
  (`self.SpawnEmitterAtTransform` "/Game/FXVarietyPack/Particles/P_ky_explosion.P_ky_explosion" (`KismetMathLibrary.MakeTransform` (.location _returnvalue) (.rotation _returnvalue) (0.3 0.3 0.3))))

(event `self.OnCreate`
  (`self.SpawnEmitterAtTransform` "/Game/FXVarietyPack/Particles/P_ky_shotShockwave.P_ky_shotShockwave"))

(event `self.ParticleSystem.OnSystemFinished`
  (params (PSystem :type "ParticleSystemComponent Object Reference"))
  (`self.SetDelayDestroy` false))

(event `self.OnDestroy`
  (bind (_returnvalue_location _returnvalue_rotation) (`KismetMathLibrary.BreakTransform` (`self.GetTransform`)))
  (`ActorComponent.Deactivate` (`self.ParticleSystem`))
  (`self.SetSpeed` 0.0)
  (`self.SpawnEmitterAtTransform` "/Game/FXVarietyPack/Particles/P_ky_explosion.P_ky_explosion" (`KismetMathLibrary.MakeTransform` _returnvalue_location _returnvalue_rotation (0.3 0.3 0.3)))
  (`self.SetActorEnableCollision` false))

(fn `UserConstructionScript`
  (`parent.UserConstructionScript`)
  (`self.AddComponentToDeactivateOnDelayedDestroy` (`self.Collision`)))