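; BP_FireNado is an area ability that sprays fireballs in random directions while it is active.
; Its update event accumulates delta time and chains a BP_Fireball every 0.2 seconds at a random angle, passing -1 for size, speed and max distance.
; The timer subtracts the interval rather than resetting, carrying leftover time forward, and fires at most once per update.
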(event `self.OnUpdate`
  (params (deltaTime :type "Float (single-precision)"))
  (bind _output_get (set `self.Timer` (+ deltaTime (`self.Timer`))))
  (if (>= _output_get 0.2)
    (`self.ChainProjectile` "/Game/KamARPG/Abilities/Projectiles/BP_Fireball.BP_Fireball_C" -1.0 (`KismetMathLibrary.RandomFloatInRange` 0.0 360.0) -1.0 -1.0)
    (set `self.Timer` (- (`self.Timer`) 0.2))))

(fn `UserConstructionScript`
  (`parent.UserConstructionScript`))