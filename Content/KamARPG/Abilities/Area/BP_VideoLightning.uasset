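; BP_VideoLightning is an area ability Blueprint that repeatedly spawns random lightning through ability chaining.
; OnUpdate accumulates delta time and chains BP_Lightning_Random each time the timer reaches a half-second interval.
; It subtracts the interval instead of resetting to zero, carrying leftover time into the next cycle.
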(event `self.OnUpdate`
  (params (deltaTime :type "Float (single-precision)"))
  (bind _output_get (set `self.Timer` (+ deltaTime (`self.Timer`))))
  (if (>= _output_get 0.5)
    (`self.ChainAbility` "/Game/KamARPG/Abilities/Targeted/BP_Lightning_Random.BP_Lightning_Random_C")
    (set `self.Timer` (- (`self.Timer`) 0.5))))

(fn `UserConstructionScript`
  (`parent.UserConstructionScript`))