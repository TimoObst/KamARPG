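; BP_Area_TargetedTimerTest is a test area ability that repeatedly chains a BP_Explosion_Closest ability while it runs.
; On tick it accumulates delta time and, whenever the timer rises above zero, fires the chained explosion and subtracts a fixed interval.
; This gives an immediate first trigger followed by evenly spaced repeats.
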(event `self.OnTick`
  (params (deltaTime :type "Float (single-precision)"))
  (bind _output_get (set `self.Timer` (+ deltaTime (`self.Timer`))))
  (if (> _output_get 0.0)
    (`self.ChainAbility` "/Game/KamARPG/Abilities/Targeted/BP_Explosion_Closest.BP_Explosion_Closest_C")
    (set `self.Timer` (- (`self.Timer`) 0.8))))

(fn `UserConstructionScript`
  (`parent.UserConstructionScript`))