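; Example RPG unit Blueprint that reacts visually to damage and tracks its hit and death state.
; On BeginPlay it binds handlers to the damage-taken and death events of BPEnemyUnit.
; Positive damage sets a material flash color by damage element, plays a timeline that animates the flash alpha on the skeletal mesh, and sets IsAttacked.
; Death only sets the IsDead flag.
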(event `self.ReceiveBeginPlay`
  (bind _bp_enemyunit (`self.BP_EnemyUnit`))
  (add `KamUnit.OnDamageTakenEvent` _bp_enemyunit (delegate `OnUnitDamageTaken`))
  (add `KamUnit.OnDeathEvent` _bp_enemyunit (delegate `OnUnitDeath`)))

(event `OnUnitDamageTaken`
  (params (damageTaken :type "Float (double-precision)") (damageElement :type "EKamElement Enum" :default "EL_True") (isCrit :type Boolean))
  (bind _skeletalmesh (`self.SkeletalMesh`))
  (if (> damageTaken 0.0)
    (switch `EKamElement` damageElement
      (:`EL_True`
        (`MeshComponent.SetVectorParameterValueOnMaterials` _skeletalmesh "FlashColor" (1.0 1.0 1.0)))
      (:`EL_Physical`
        (`MeshComponent.SetVectorParameterValueOnMaterials` _skeletalmesh "FlashColor" (1.0 0.0 0.0)))
      (:`EL_Magic`
        (`MeshComponent.SetVectorParameterValueOnMaterials` _skeletalmesh "FlashColor" (1.0 0.0 1.0)))
      (:`EL_Fire`
        (`MeshComponent.SetVectorParameterValueOnMaterials` _skeletalmesh "FlashColor" (10.0 0.0 0.0))))
    (`self.FlashColor`)
    (set `self.IsAttacked` true)))

(event `OnUnitDeath`
  (set `self.IsDead` true))

(event `FlashColor`
  (bind (_direction _alpha) (`Timeline|FlashColorTimeline` :!via `PlayFromStart`)
    (:`Update`
      (`MeshComponent.SetScalarParameterValueOnMaterials` (`self.SkeletalMesh`) "FlashAlpha" _alpha))))

(fn `UserConstructionScript`)