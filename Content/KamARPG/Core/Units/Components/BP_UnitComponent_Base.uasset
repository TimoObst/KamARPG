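; Base unit component for KamARPG that handles combat math and death, making the owner unhittable and destroying it after a short delay.
; Damage reduction passes True damage through, chains Armor or MagicResist into ResistAll for Physical or Magic, and applies only ResistAll to Fire.
; Each step multiplies damage by stat / (stat + attacker level × factor).
; Crit chance divides the CritChance attribute by a cost growing exponentially with level, feeding a random crit roll.
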(event `self.OnDeath`
  (set `self.isHittable` false)
  (`KismetSystemLibrary.Delay` 1.0)
  (`Actor.K2_DestroyActor` (`self.owner`)))

(event `self.OnDamageTaken`
  (params (DamageTaken :type "Float (single-precision)") (damageType :type "EKamElement Enum" :default "EL_True") (isCriticalHit :type Boolean)))

(fn `CalculateCritChance`
  (returns (ReturnValue :type "Float (double-precision)"))
  (locals (CritChance :type "Float (double-precision)") (CritNeededPerPercent :type "Float (double-precision)") (GrowthPerLevel :type "Float (double-precision)"))
  ;[1 1 1] Initialize Values
  (set `local.CritNeededPerPercent` 10.0)
  (set `local.CritChance` 0.0)
  (set `local.GrowthPerLevel` 1.05)
  ;[1 1 1] Calculate Crit needed from Level
  (bind _returnvalue (`self.GetAttribute` "AT_Level"))
  (set `local.CritNeededPerPercent` (* (`KismetMathLibrary.MultiplyMultiply_FloatFloat` (`local.GrowthPerLevel`) (`KismetMathLibrary.Conv_IntToDouble` _returnvalue)) (`local.CritNeededPerPercent`)))
  ;[1 1 1] Calculate Crit Chance
  (bind _returnvalue_2 (`self.GetAttribute` "AT_CritChance"))
  (bind _output_get (set `local.CritChance` (/ (`KismetMathLibrary.Conv_IntToDouble` _returnvalue_2) (`local.CritNeededPerPercent`))))
  (return _output_get))

(fn `CalculateDamageReduction`
  (params (damageIn :type "Float (double-precision)") (caster :type "KamUnitSnapshot Object Reference") (damageType :type "EKamElement Enum" :default "EL_True"))
  (returns (ReturnValue :type "Float (double-precision)"))
  (switch `EKamElement` damageType
    (:`EL_True`
      (return damageIn))
    (:`EL_Physical`
      (bind _damage_out (`self.PhysicalDamageReduction` damageIn caster)
        (:`Exec Out`
          (bind _damage_out_2 (`self.AllResistDamageReduction` _damage_out caster)
            (:`Exec out`
              (return _damage_out_2))))))
    (:`EL_Magic`
      (bind _damage_out_3 (`self.MagicDamageReduction` damageIn caster)
        (:`Exec Out`
          (bind _damage_out_4 (`self.AllResistDamageReduction` _damage_out_3 caster)
            (:`Exec out`
              (return _damage_out_4))))))
    (:`EL_Fire`
      (bind _damage_out_5 (`self.AllResistDamageReduction` damageIn caster)
        (:`Exec out`
          (return _damage_out_5))))))

(fn `DamageHasCrit`
  (params (critChance :type "Float (double-precision)") (caster :type "KamUnitSnapshot Object Reference") (damageType :type "EKamElement Enum" :default "EL_True"))
  (returns (ReturnValue :type Boolean))
  (return (> (+ critChance (`KamUnitSnapshot.GetCritChance` caster)) (`KismetMathLibrary.RandomFloatInRange` 0.0 100.0))))

(fn `UserConstructionScript`)